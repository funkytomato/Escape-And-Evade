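; Menu player pawn that moves through the character selection screen, sliding between preset viewpoints for five selectable characters.
; MoveLeft and MoveRight step a bounded index, which picks a per-character timeline that lerps the pawn's transform toward that character's stored transform.
; After a short delay it passes the index to the selection widget to update the displayed name, then re-enables clicking.
; GoToCharacterSelect plays a timeline that drives the same move and name update.
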(event Custom|GoToCharacterSelect
  (bind _arrowcount (Variables|Default|GetArrowCount))
  ;[1 1 1] Animate to Player selected character, and show the selection menu
  (bind _alpha (Timeline|CharacterSelect Play)
    (:Update
      (CallFunction|PlayerCharacterTimeline _arrowcount)
      (CallFunction|UpdateCharacterName _arrowcount))))

(event Custom|MoveRight
  ;[1 1 1] Move the character selection left or right, and update the view, and character name
  (if (< (Variables|Default|GetArrowCount) (Variables|Default|GetCharacterTypeNumber))
    (Variables|Default|SetCanClick? false)
    (Variables|Default|SetArrowCount (Math|Integer|Clamp(Integer) (+ (Variables|Default|GetArrowCount) 1) 0 (Variables|Default|GetCharacterTypeNumber)))
    (CallFunction|PlayerCharacterTimeline (Variables|Default|GetArrowCount))
    (Utilities|FlowControl|Delay 0.5)
    (CallFunction|UpdateCharacterName (Variables|Default|GetArrowCount))
    (else
      (Development|PrintString "Move right exceeded"))))

(event Custom|MoveLeft
  ;[1 1 1] Move the character selection left or right, and update the view, and character name
  (if (> (Variables|Default|GetArrowCount) 0)
    (Variables|Default|SetCanClick? false)
    (Variables|Default|SetArrowCount (Math|Integer|Clamp(Integer) (- (Variables|Default|GetArrowCount) 1) 0 (Variables|Default|GetCharacterTypeNumber)))
    (CallFunction|PlayerCharacterTimeline (Variables|Default|GetArrowCount))
    (Utilities|FlowControl|Delay 0.5)
    (CallFunction|UpdateCharacterName (Variables|Default|GetArrowCount))
    (else
      (Development|PrintString "MoveLeft exceeded"))))

(event Custom|PlayerCharacterTimeline
  (params (Arrow :type Integer))
  ;[1 1 1] Animate to the selected character location
  (switch int Arrow
    (:0
      (bind _alpha (Timeline|BusinessManInShirtTimeline Play)
        (:Update
          (CallFunction|UpdateTransform (Variables|Default|GetBusinessManInShirtTransform) _alpha))))
    (:1
      (bind _alpha_2 (Timeline|BusinessWomanTimeline Play)
        (:Update
          (CallFunction|UpdateTransform (Variables|Default|GetBusinessWomanTransform) _alpha_2))))
    (:2
      (bind _alpha_3 (Timeline|DaughterTimeline Play)
        (:Update
          (CallFunction|UpdateTransform (Variables|Default|GetDaughterTransform) _alpha_3))))
    (:3
      (bind _alpha_4 (Timeline|WomanInRedTimeline Play)
        (:Update
          (CallFunction|UpdateTransform (Variables|Default|GetWomanInRedTransform) _alpha_4))))
    (:4
      (bind _alpha_5 (Timeline|SchoolBoyTimeline Play)
        (:Update
          (CallFunction|UpdateTransform (Variables|Default|GetSchoolBoyTransform) _alpha_5))))))

(event Custom|UpdateCharacterName
  (params (Arrow :type Integer))
  ;[1 1 1] Update the character name
  (bind _ascharacter_select_wbp (Utilities|Casting|CastToCharacterSelect_WBP (Variables|Default|GetCharacterSelectionWB_Ref))
    (:then
      (Default|CallUpdateCharacterNameMsg _ascharacter_select_wbp Arrow)
      (Variables|Default|SetCanClick? true))
    (:CastFailed
      (Development|PrintString "MyPlayerPawn failed to cast"))))

(event Custom|UpdateTransform
  (params (NewTransform :type Transform) (Alpha :type Float%20%28single-precision%29))
  ;[1 1 1] Update the character location
  (Transformation|SetActorTransform (Math|Transform|Lerp(Transform) (Transformation|GetActorTransform) NewTransform Alpha)))

(event EventBeginPlay
  ;[1 1 1] On Begin, get GameInstance and Show the main menu
  (bind _asescape_and_evade_game_instance (Utilities|Casting|CastToEscapeAndEvadeGameInstance (Game|GetGameInstance)))
  (Variables|Default|SetGameInstanceRef _asescape_and_evade_game_instance))

(fn ConstructionScript)