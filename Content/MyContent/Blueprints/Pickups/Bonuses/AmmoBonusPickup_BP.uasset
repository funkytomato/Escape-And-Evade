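; A bonus ammo pickup that grants ammo to the player character when touched.
; When its collision component overlaps a MasterCharacter, it calls that character's bonus ammo message with the pickup's ammo type and boost amount.
; It then destroys itself and plays a coin sound at its location; other overlapping actors are ignored.
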(event OnComponentBeginOverlap(Collision)
  (params (OverlappedComponent :type Primitive%20Component%20Object%20Reference) (OtherActor :type Actor%20Object%20Reference) (OtherComp :type Primitive%20Component%20Object%20Reference) (OtherBodyIndex :type Integer) (bFromSweep :type Boolean) (SweepResult :type Hit%20Result%20Structure%20%28by%20ref%29))
  (bind _asmaster_character (Utilities|Casting|CastToMasterCharacter OtherActor))
  (Default|CallBonusAmmoMessage _asmaster_character (Variables|Default|GetAmmoType) (Variables|Default|GetBoostAmount))
  (Actor|DestroyActor)
  (Audio|PlaySoundatLocation "/Game/Ultimate_SFX/Hero_Voice_Jack/Wavs/Coin.Coin" (Transformation|GetActorLocation) "0, 0, 0" 1.0 1.0 0.0 0 0 0))

(event EventBeginPlay
  (|CallParentFunction) ; This node is disabled and will not be called.\nDrag off pins to build functionality.
)

(event Collision|EventActorBeginOverlap
  (params (OtherActor :type Actor%20Object%20Reference))
  (|CallParentFunction OtherActor) ; This node is disabled and will not be called.\nDrag off pins to build functionality.
)

(event EventTick
  (params (DeltaSeconds :type Float%20%28single-precision%29))
  (|CallParentFunction DeltaSeconds) ; This node is disabled and will not be called.\nDrag off pins to build functionality.
)

(fn ConstructionScript
  (|CallParentFunction))