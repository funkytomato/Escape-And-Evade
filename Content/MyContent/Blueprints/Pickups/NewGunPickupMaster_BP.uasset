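; Master Blueprint for gun pickups that characters collect by walking into a collision sphere.
; On BeginPlay it looks up its gun type in the weapon info data table and caches whether it is a longarm.
; On overlap with a MasterCharacter not carrying a longarm, it sends the gun type to that character and destroys itself.
; The cached longarm flag is not used in the overlap check.
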(event OnComponentBeginOverlap(CollisionSphere)
  (params (OverlappedComponent :type Primitive%20Component%20Object%20Reference) (OtherActor :type Actor%20Object%20Reference) (OtherComp :type Primitive%20Component%20Object%20Reference) (OtherBodyIndex :type Integer) (bFromSweep :type Boolean) (SweepResult :type Hit%20Result%20Structure%20%28by%20ref%29))
  (bind _asmaster_character (Utilities|Casting|CastToMasterCharacter OtherActor))
  ;[1 1 1] Carrying Longarm?
  (if (not (Variables|/Game/MyContent/Blueprints/Characters/MasterCharacter.MasterCharacter_C|GetHasLongArm? _asmaster_character))
    ;[1 1 1] Pickup gun
    (Default|CallGunPickedUpMessage _asmaster_character (Variables|Default|GetGunTypeName))
    (Actor|DestroyActor)))

(event EventBeginPlay
  (bind _returnvalue (Utilities|GetDataTableRow "/Game/MyContent/Blueprints/Weapons/Welded/WeaponInfoTable.WeaponInfoTable" (Variables|Default|GetGunTypeName))
    (:then
      (Variables|Default|SetIsLongarm? (.IsLongarm (Utilities|Struct|BreakWeaponInfoStruct _returnvalue))))))

(fn ConstructionScript)