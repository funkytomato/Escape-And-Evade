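; PickupMaster_BP is a pickup, apparently the base for others, that hands its item to the player on interaction.
; Interact checks CanPickup, casts player 0 to MasterCharacter and calls that character's PickedUpItem dispatcher with ItemType and PickupClassType.
; It then destroys itself and plays a coin pickup sound at the character's location.
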(event EventInteract
  (if (Variables|Default|GetCanPickup)
    (bind _asmaster_character (Utilities|Casting|CastToMasterCharacter (Game|GetPlayerCharacter 0)))
    (if true
      (Default|CallPickedUpItem _asmaster_character (Variables|Default|GetItem%20Type) (Variables|Default|GetPickupClassType))
      (Actor|DestroyActor)
      (Audio|PlaySoundatLocation "/Game/Ultimate_SFX/Ultimate_Retro_Sounds/Wavs/Coin_Pickup_-_50/Coin_Pickup_15.Coin_Pickup_15" (Transformation|GetActorLocation _asmaster_character) "0, 0, 0" 1.0 1.0 0.0 0 0 0))))

(fn ConstructionScript)