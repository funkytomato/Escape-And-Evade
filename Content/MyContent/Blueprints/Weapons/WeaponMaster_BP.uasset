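; WeaponMaster_BP is a weapon Blueprint, apparently a master class, that can display as either a skeletal or a static mesh.
; ShowSkeletalMesh and ShowStaticMesh toggle visibility between the two components without propagating to children.
; A WeaponType switch maps Throwable to the static mesh, with a debug print, and other types to the skeletal mesh.
; That switch is unconnected and never runs; BeginPlay and the construction script are empty.
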(event EventBeginPlay)

(fn ConstructionScript)

(fn ShowSkeletalMesh
  ;[1 1 1] Show Skeletal Mesh
  (Rendering|SetVisibility (Variables|Default|GetSkeletalMesh) true false)
  (Rendering|SetVisibility (Variables|Default|GetStaticMesh) false false))

(fn ShowStaticMesh
  ;[1 1 1] Show Static Mesh
  (Rendering|SetVisibility (Variables|Default|GetSkeletalMesh) false false)
  (Rendering|SetVisibility (Variables|Default|GetStaticMesh) true false))