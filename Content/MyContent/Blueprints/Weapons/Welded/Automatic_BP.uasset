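; Automatic weapon Blueprint that adds hold-to-fire behavior to a parent weapon class.
; StartShooting calls the parent, fires a projectile immediately, then starts a looping timer on FireProjectile at the FireRate interval.
; StopShooting calls the parent and clears the stored GunTimer handle to end the burst, so firing needs no Tick logic.
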(event EventBeginPlay
  (|CallParentFunction) ; This node is disabled and will not be called.\nDrag off pins to build functionality.
)

(event Collision|EventActorBeginOverlap
  (params (OtherActor :type Actor%20Object%20Reference))
  (|CallParentFunction OtherActor) ; This node is disabled and will not be called.\nDrag off pins to build functionality.
)

(event EventTick
  (params (DeltaSeconds :type Float%20%28single-precision%29))
  (|CallParentFunction DeltaSeconds) ; This node is disabled and will not be called.\nDrag off pins to build functionality.
)

(event EventStartShooting
  (|CallParentFunction)
  (CallFunction|FireProjectile)
  (bind _returnvalue (Utilities|Time|SetTimerbyFunctionName 0 "FireProjectile" (Variables|Default|GetFireRate) true))
  (Variables|Default|SetGunTimer _returnvalue))

(event EventStopShooting
  (|CallParentFunction)
  (Utilities|Time|ClearandInvalidateTimerbyHandle (Variables|Default|GetGunTimer)))

(fn ConstructionScript
  (|CallParentFunction))