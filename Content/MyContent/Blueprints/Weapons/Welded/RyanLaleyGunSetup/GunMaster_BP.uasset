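; Base gun for a MasterCharacter parent actor, managing firing state, clip and reserve ammo, and reloading.
; FireProjectile either runs a hitscan multi-line trace or spawns a projectile, then decrements ammo and signals the owner when empty.
; Projectile shots also run a forward sphere trace that calls Threatened on a character it hits.
; Hitscan hits feed SpawnDecal, but its random surface-based decal logic is disconnected and never runs.
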(event Custom|StartShooting
  (Variables|Default|SetIsFiring? true))

(event Custom|StopShooting
  (Variables|Default|SetIsFiring? false))

(event EventBeginPlay
  (|CallParentFunction) ; This node is disabled and will not be called.\nDrag off pins to build functionality.
)

(event Collision|EventActorBeginOverlap
  (params (OtherActor :type Actor%20Object%20Reference))
  (|CallParentFunction OtherActor) ; This node is disabled and will not be called.\nDrag off pins to build functionality.
)

(event EventTick
  (params (DeltaSeconds :type Float%20%28single-precision%29))
  (|CallParentFunction DeltaSeconds) ; This node is disabled and will not be called.\nDrag off pins to build functionality.
)

(fn ConstructionScript
  (|CallParentFunction))

(fn ThreatTrace
  (params (Radius :type Float%20%28single-precision%29))
  (bind _barrel_rp (Variables|Default|GetBarrel_RP))
  (bind _returnvalue (Transformation|GetWorldLocation _barrel_rp))
  (bind _asmaster_character (Utilities|Casting|CastToMasterCharacter (Actor|GetParentActor)))
  (bind _outhit (Collision|SphereTraceByChannel _returnvalue (+ _returnvalue (* (Math|Vector|GetForwardVector (Transformation|GetWorldRotation (Variables|/Script/Engine.Character|GetCapsuleComponent _asmaster_character))) (Variables|Default|GetRange))) Radius "TraceTypeQuery2" false (Utilities|Array|MakeArray 0) "None" true "(R=0.009268,G=0.021773,B=1.000000,A=1.000000)" "(R=0.000000,G=0.795357,B=1.000000,A=1.000000)"))
  (if (.bblockinghit _outhit)
    (bind _asmaster_character_2 (Utilities|Casting|CastToMasterCharacter (.hitactor _outhit)))
    (Default|Threatened _asmaster_character_2)))

(fn Reload
  (Variables|Default|SetBulletDifference (- (Variables|Default|GetClipSize) (Variables|Default|GetAmmoCount)))
  (if (>= (Variables|Default|GetAmmoMax) (Variables|Default|GetBulletDifference))
    (Variables|Default|SetAmmoCount (Variables|Default|GetClipSize))
    (Variables|Default|SetAmmoMax (- (Variables|Default|GetAmmoMax) (Variables|Default|GetBulletDifference)))
    (else
      (Variables|Default|SetAmmoCount (+ (Variables|Default|GetAmmoCount) (Variables|Default|GetAmmoMax)))
      (Variables|Default|SetAmmoMax 0))))

(fn FireProjectile
  (bind _asmaster_character (Utilities|Casting|CastToMasterCharacter (Actor|GetParentActor)))
  (Variables|Default|SetGunOwner _asmaster_character)
  (if (Variables|/Game/MyContent/Blueprints/Characters/MasterCharacter.MasterCharacter_C|GetCanShoot? _asmaster_character)
    (if (Variables|Default|GetIsHitScan)
      (if (> (Variables|Default|GetAmmoCount) 0)
        (if true
          (Variables|Default|SetGunDirection (Math|Vector|GetForwardVector (Transformation|GetWorldRotation (Variables|/Script/Engine.Character|GetCapsuleComponent (Variables|Default|GetGunOwner)))))
          (bind _outhits (Collision|MultiLineTraceByChannel (Transformation|GetWorldLocation (Variables|Default|GetBarrel_RP)) (+ (Transformation|GetWorldLocation (Variables|/Script/Engine.Character|GetCapsuleComponent (Variables|Default|GetGunOwner))) (* (Math|Vector|GetForwardVector (Transformation|GetWorldRotation (Variables|/Script/Engine.Character|GetCapsuleComponent (Variables|Default|GetGunOwner)))) 2e+03)) "TraceTypeQuery1" false 0 "ForOneFrame"))
          (CallFunction|ProcessHits _outhits)
          (Utilities|SpawnDecal)
          (if true
            (Physics|AddImpulseatLocation (* (Variables|Default|GetGunDirection) 2e+05) "0, 0, 0" "None"))
          (bind _result (Math|Integer|DecrementInt (Variables|Default|GetAmmoCount) :!label _label)
            (:%20%20
              (if (not (> _result 0))
                (CallFunction|StopShooting)
                (Default|GunEmptyEvent (Variables|Default|GetGunOwner)))))))
      (elif (> (Variables|Default|GetAmmoCount) 0)
        (Game|SpawnActorfromClass "/Game/MyContent/Blueprints/Projectiles/FirstPersonProjectile.FirstPersonProjectile_C" (Math|Transform|MakeTransform (Transformation|GetWorldLocation (Variables|Default|GetBarrel_RP)) (Transformation|GetWorldRotation (Variables|/Script/Engine.Character|GetCapsuleComponent (Variables|Default|GetGunOwner))) "1,1,1") "AlwaysSpawn" 0 (Variables|Default|GetGunOwner))
        (CallFunction|ThreatTrace (Variables|Default|GetThreatLevel))
        (goto _label)))))

(fn IncreaseAmmo
  (params (amount :type Integer))
  (Variables|Default|SetAmmoMax (+ (Variables|Default|GetAmmoMax) amount)))

(fn GetImpactDecal
  (params (SurfaceType :type EPhysicalSurface%20Enum :default "SurfaceType_Default"))
  (bind _grassdecals (LocalVariables|GetGrassDecals))
  (bind _wooddecals (LocalVariables|GetWoodDecals))
  (bind _concretedecals (LocalVariables|GetConcreteDecals))
  (bind _graveldecals (LocalVariables|GetGravelDecals))
  (bind _fleshdecals (LocalVariables|GetFleshDecals))
  (bind _rockdecals (LocalVariables|GetRockDecals))
  (bind _waterdecals (LocalVariables|GetWaterDecals))
  (bind _electricaldecals (LocalVariables|GetElectricalDecals))
  (bind _defaultdecals (LocalVariables|GetDefaultDecals))
  (bind _rustdecals (LocalVariables|GetRustDecals))
  (bind _glassdecals (LocalVariables|GetGlassDecals))
  (switch Utilities|FlowControl|Switch|SwitchonEPhysicalSurface SurfaceType
    (:SurfaceType_Default
      (LocalVariables|SetSelectedDecal (Utilities|Array|Get(acopy) _defaultdecals (Math|Random|RandomIntegerinRange 0 (- (Utilities|Array|Length _defaultdecals) 1)))))
    (:SurfaceType1
      (LocalVariables|SetSelectedDecal (Utilities|Array|Get(acopy) _grassdecals (Math|Random|RandomIntegerinRange 0 (- (Utilities|Array|Length _grassdecals) 1)))))
    (:SurfaceType2
      (LocalVariables|SetSelectedDecal (Utilities|Array|Get(acopy) _wooddecals (Math|Random|RandomIntegerinRange 0 (- (Utilities|Array|Length _wooddecals) 1)))))
    (:SurfaceType3
      (LocalVariables|SetSelectedDecal (Utilities|Array|Get(acopy) _concretedecals (Math|Random|RandomIntegerinRange 0 (- (Utilities|Array|Length _concretedecals) 1)))))
    (:SurfaceType4
      (LocalVariables|SetSelectedDecal (Utilities|Array|Get(acopy) _graveldecals (Math|Random|RandomIntegerinRange 0 (- (Utilities|Array|Length _graveldecals) 1)))))
    (:SurfaceType5
      (LocalVariables|SetSelectedDecal (Utilities|Array|Get(acopy) _fleshdecals (Math|Random|RandomIntegerinRange 0 (- (Utilities|Array|Length _fleshdecals) 1)))))
    (:SurfaceType6
      (LocalVariables|SetSelectedDecal (Utilities|Array|Get(acopy) _rockdecals (Math|Random|RandomIntegerinRange 0 (- (Utilities|Array|Length _rockdecals) 1)))))
    (:SurfaceType7
      (LocalVariables|SetSelectedDecal (Utilities|Array|Get(acopy) _waterdecals (Math|Random|RandomIntegerinRange 0 (- (Utilities|Array|Length _waterdecals) 1)))))
    (:SurfaceType8
      (LocalVariables|SetSelectedDecal (Utilities|Array|Get(acopy) _electricaldecals (Math|Random|RandomIntegerinRange 0 (- (Utilities|Array|Length _electricaldecals) 1)))))
    (:SurfaceType9
      (LocalVariables|SetSelectedDecal (Utilities|Array|Get(acopy) _rustdecals (Math|Random|RandomIntegerinRange 0 (- (Utilities|Array|Length _rustdecals) 1)))))
    (:SurfaceType10
      (LocalVariables|SetSelectedDecal (Utilities|Array|Get(acopy) _glassdecals (Math|Random|RandomIntegerinRange 0 (- (Utilities|Array|Length _glassdecals) 1))))))
  (return (LocalVariables|GetSelectedDecal)))

(fn ProcessHits
  (params (HitResults :type Array%20of%20Hit%20Result%20Structures))
  (for _array_element HitResults
    (Utilities|SpawnDecal (.HitActor (Collision|BreakHitResult _array_element)) (.ImpactPoint (Collision|BreakHitResult _array_element)) (.ImpactNormal (Collision|BreakHitResult _array_element)) (.HitBoneName (Collision|BreakHitResult _array_element)) (.PhysMat (Collision|BreakHitResult _array_element))))
  (return))