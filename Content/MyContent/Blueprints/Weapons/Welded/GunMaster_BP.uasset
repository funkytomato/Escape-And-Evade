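; GunMaster_BP is a gun actor, parented to a MasterCharacter, that handles firing, ammo and reloading.
; FireProjectile either line-traces from the follow camera to push physics objects, or spawns a projectile at the barrel and spends ammo.
; Projectile shots also sphere-trace along the camera's aim to call Threatened on a character in the way.
; Reload refills the clip from reserve ammo, while Start/StopShooting only toggle IsFiring.
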(event Custom|StartShooting
  (Variables|Default|SetIsFiring? true))

(event Custom|StopShooting
  (Variables|Default|SetIsFiring? false))

(event EventBeginPlay
  (|CallParentFunction) ; This node is disabled and will not be called.\nDrag off pins to build functionality.
)

(event Collision|EventActorBeginOverlap
  (params (OtherActor :type Actor%20Object%20Reference))
  (|CallParentFunction OtherActor) ; This node is disabled and will not be called.\nDrag off pins to build functionality.
)

(event EventTick
  (params (DeltaSeconds :type Float%20%28single-precision%29))
  (|CallParentFunction DeltaSeconds) ; This node is disabled and will not be called.\nDrag off pins to build functionality.
)

(fn ConstructionScript
  (|CallParentFunction))

(fn ThreatTrace
  (params (InputPin :type Float%20%28single-precision%29))
  (bind _barrel_rp (Variables|Default|GetBarrel_RP))
  (bind _returnvalue (Transformation|GetWorldLocation _barrel_rp))
  (bind _asmaster_character (Utilities|Casting|CastToMasterCharacter (Actor|GetParentActor)))
  (bind _outhit (Collision|SphereTraceByChannel _returnvalue (+ _returnvalue (* (Math|Vector|GetForwardVector (Transformation|GetWorldRotation (Variables|/Game/MyContent/Blueprints/Characters/MasterCharacter.MasterCharacter_C|GetFollowCamera _asmaster_character))) (Variables|Default|GetRange))) 0.0 "TraceTypeQuery2" false (Utilities|Array|MakeArray 0) "ForDuration" true "(R=0.009268,G=0.021773,B=1.000000,A=1.000000)" "(R=0.000000,G=0.795357,B=1.000000,A=1.000000)"))
  (if (.bblockinghit _outhit)
    (bind _asmaster_character_2 (Utilities|Casting|CastToMasterCharacter (.hitactor _outhit)))
    (Default|Threatened _asmaster_character_2)))

(fn Reload
  (Variables|Default|SetBulletDifference (- (Variables|Default|GetClipSize) (Variables|Default|GetAmmoCount)))
  (if (>= (Variables|Default|GetAmmoMax) (Variables|Default|GetBulletDifference))
    (Variables|Default|SetAmmoCount (Variables|Default|GetClipSize))
    (Variables|Default|SetAmmoMax (- (Variables|Default|GetAmmoMax) (Variables|Default|GetBulletDifference)))
    (else
      (Variables|Default|SetAmmoCount (+ (Variables|Default|GetAmmoCount) (Variables|Default|GetAmmoMax)))
      (Variables|Default|SetAmmoMax 0))))

(fn FireProjectile
  (bind _asmaster_character (Utilities|Casting|CastToMasterCharacter (Actor|GetParentActor)))
  (Variables|Default|SetGunOwner _asmaster_character)
  (if (Variables|Default|GetIsHitScan)
    (if (> (Variables|Default|GetAmmoCount) 0)
      (if true
        (Variables|Default|SetGunDirection (Math|Vector|GetForwardVector (Transformation|GetWorldRotation (Variables|/Game/MyContent/Blueprints/Characters/MasterCharacter.MasterCharacter_C|GetFollowCamera (Variables|Default|GetGunOwner)))))
        (bind _outhit (Collision|LineTraceByChannel (Transformation|GetWorldLocation (Variables|/Game/MyContent/Blueprints/Characters/MasterCharacter.MasterCharacter_C|GetFollowCamera (Variables|Default|GetGunOwner))) (+ (Transformation|GetWorldLocation (Variables|/Game/MyContent/Blueprints/Characters/MasterCharacter.MasterCharacter_C|GetFollowCamera (Variables|Default|GetGunOwner))) (* (Math|Vector|GetForwardVector (Transformation|GetWorldRotation (Variables|/Game/MyContent/Blueprints/Characters/MasterCharacter.MasterCharacter_C|GetFollowCamera (Variables|Default|GetGunOwner)))) 2e+03)) "TraceTypeQuery1" false 0 "ForDuration"))
        (if (.bBlockingHit (Collision|BreakHitResult _outhit))
          (if (Physics|IsSimulatingPhysics (.HitComponent (Collision|BreakHitResult _outhit)) "None")
            (Physics|AddImpulseatLocation (.HitComponent (Collision|BreakHitResult _outhit)) (* (Variables|Default|GetGunDirection) 2e+05) (.ImpactPoint (Collision|BreakHitResult _outhit)) "None")))))
    (elif (> (Variables|Default|GetAmmoCount) 0)
      (Game|SpawnActorfromClass "/Game/MyContent/Blueprints/Projectiles/FirstPersonProjectile.FirstPersonProjectile_C" (Math|Transform|MakeTransform (Transformation|GetWorldLocation (Variables|Default|GetBarrel_RP)) (Transformation|GetWorldRotation (Variables|/Script/Engine.Character|GetCapsuleComponent (Variables|Default|GetGunOwner))) "1,1,1") "AlwaysSpawn" 0 (Variables|Default|GetGunOwner))
      (CallFunction|ThreatTrace (Variables|Default|GetThreatLevel))
      (Math|Integer|DecrementInt (Variables|Default|GetAmmoCount)))))